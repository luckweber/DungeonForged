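; BP_DummyCharacter is a character Blueprint that switches between movement gaits, starting in a default gait on BeginPlay.
; Holding the 2 key applies an alternate gait, and releasing it restores the previously stored one.
; UpdateGait records current and previous gaits, passes the new one to the Anim Instance, and copies speed, acceleration and braking values from the GaitSettings map into CharacterMovement.
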(event `self.ReceiveBeginPlay`
  (`self.UpdateGait` "NewEnumerator1"))

(event `Key|Two`
  (params (Key :type "Key Structure"))
  (:`Pressed`
    (`self.UpdateGait` "NewEnumerator0"))
  (:`Released`
    (`self.UpdateGait` (`self.PreviousGait`))))

(fn `UpdateGait`
  (params (DesireGait :type "/Game/DungeonForged/Character/Dummy/E_Gaits Enum" :default "NewEnumerator0"))
  (bind _charactermovement (`self.CharacterMovement`))
  (bind (_maxwalkingspeed _maxacceleration _breakingdeceleration _breakingfrictionfactor _useseparatefriction _breakingfriction) (break `/Game/DungeonForged/Character/Dummy/F_GaitsSettings` (`BlueprintMapLibrary.Map_Find` (`self.GaitSettings`) (`local.DesireGait`))))
  (set `self.PreviousGait` (`self.CurrentGait`))
  (set `self.CurrentGait` DesireGait)
  (message `/Game/DungeonForged/Character/Dummy/BPI_Gait.ReceiveGaitData` (`SkeletalMeshComponent.GetAnimInstance` (`self.Mesh`)) DesireGait)
  (set `CharacterMovementComponent.MaxWalkSpeed` _maxwalkingspeed _charactermovement)
  (set `CharacterMovementComponent.MaxAcceleration` _maxacceleration _charactermovement)
  (set `CharacterMovementComponent.BrakingDecelerationWalking` _breakingdeceleration _charactermovement)
  (set `CharacterMovementComponent.BrakingFrictionFactor` _breakingfrictionfactor _charactermovement)
  (set `CharacterMovementComponent.bUseSeparateBrakingFriction` _useseparatefriction _charactermovement)
  (set `CharacterMovementComponent.BrakingFriction` _breakingfriction _charactermovement))

(fn `UserConstructionScript`)